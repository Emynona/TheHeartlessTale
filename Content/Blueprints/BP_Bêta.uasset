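; BP_Bêta is an interactable actor that changes the current objective to leaving the laboratory ("Sortir du laboratoire").
; A box trigger shows its text render on overlap and hides it when the overlap ends.
; Interact writes the objective to GI_HeartlessTale, then refreshes the player character's objectives widget and plays its update animation.
; Two leftover chains that set the same objective are never run.
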(event OnComponentBeginOverlap(Box)
  (params (OverlappedComponent :type Primitive%20Component%20Object%20Reference) (OtherActor :type Actor%20Object%20Reference) (OtherComp :type Primitive%20Component%20Object%20Reference) (OtherBodyIndex :type Integer) (bFromSweep :type Boolean) (SweepResult :type Hit%20Result%20Structure%20%28by%20ref%29))
  (Rendering|SetVisibility (Variables|Default|GetTextRender) true false))

(event OnComponentEndOverlap(Box)
  (params (OverlappedComponent :type Primitive%20Component%20Object%20Reference) (OtherActor :type Actor%20Object%20Reference) (OtherComp :type Primitive%20Component%20Object%20Reference) (OtherBodyIndex :type Integer))
  (Rendering|SetVisibility (Variables|Default|GetTextRender) false false))

(event EventBeginPlay)

(event Collision|EventActorBeginOverlap
  (params (OtherActor :type Actor%20Object%20Reference)))

(event EventTick
  (params (DeltaSeconds :type Float%20%28single-precision%29)))

(event EventInteract
  (bind _asbp_third_person_character (Utilities|Casting|CastToBP_ThirdPersonCharacter (Game|GetPlayerCharacter 0)))
  (bind _asgi_heartless_tale (Utilities|Casting|CastToGI_HeartlessTale (Game|GetGameInstance)))
  (Variables|/Game/Blueprints/GI_HeartlessTale.GI_HeartlessTale_C|SetObjectifs _asgi_heartless_tale "Sortir du laboratoire")
  (Default|SetObjectif (Variables|/Game/ThirdPerson/Blueprints/BP_ThirdPersonCharacter.BP_ThirdPersonCharacter_C|GetWBP_Objectives _asbp_third_person_character))
  (UserInterface|Animation|PlayAnimation (Variables|/Game/ThirdPerson/Blueprints/BP_ThirdPersonCharacter.BP_ThirdPersonCharacter_C|GetWBP_Objectives _asbp_third_person_character) (Variables|/Game/UI/Blueprints/WBP_Objectives.WBP_Objectives_C|GetUpdateObjective (Variables|/Game/ThirdPerson/Blueprints/BP_ThirdPersonCharacter.BP_ThirdPersonCharacter_C|GetWBP_Objectives _asbp_third_person_character)) 0.0 1 "Forward" 1.0 false))

(fn ConstructionScript)