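; BP_Poupee is an interactable actor, named as a doll, that opens a choice moment when the player interacts with it.
; Interact blends the player's view to the actor, then creates and displays the WBP_Choix1 widget.
; It also sets the ThirdChoice flag on GI_HeartlessTale, so the game instance records that this choice was reached.
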(event EventBeginPlay)

(event Collision|EventActorBeginOverlap
  (params (OtherActor :type Actor%20Object%20Reference)))

(event EventTick
  (params (DeltaSeconds :type Float%20%28single-precision%29)))

(event EventInteract
  (Utilities|FlowControl|Sequence
    (:then_0
      (Game|Player|SetViewTargetwithBlend (Game|GetPlayerController 0) self 2.0 "VTBlend_Linear" 0.0 false))
    (:then_1
      (bind _returnvalue (UserInterface|CreateWidget "/Game/UI/WBP_Choix1.WBP_Choix1_C"))
      (UserInterface|Viewport|AddtoViewport _returnvalue 0)
      (bind _asgi_heartless_tale (Utilities|Casting|CastToGI_HeartlessTale (Game|GetGameInstance)))
      (Variables|/Game/Blueprints/GI_HeartlessTale.GI_HeartlessTale_C|SetThirdChoice _asgi_heartless_tale true))))

(fn ConstructionScript
  (|CallParentFunction))