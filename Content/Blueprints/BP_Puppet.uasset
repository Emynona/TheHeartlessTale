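; BP_Puppet is an interactable lab keepsake that reflects the player's third story choice, showing either a doll or a flower.
; On BeginPlay it reads GI_HeartlessTale and, once that choice is made, spawns a point light and matching mesh.
; Its box overlap toggles input and an E prompt.
; Interacting toggles a character input lock, a camera blend to the actor and a text widget describing the object.
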(event OnComponentBeginOverlap(Box)
  (params (OverlappedComponent :type Primitive%20Component%20Object%20Reference) (OtherActor :type Actor%20Object%20Reference) (OtherComp :type Primitive%20Component%20Object%20Reference) (OtherBodyIndex :type Integer) (bFromSweep :type Boolean) (SweepResult :type Hit%20Result%20Structure%20%28by%20ref%29))
  ;[1 1 1] Zone dans laquelle linteraction est possible
  (if (Variables|/Game/Blueprints/GI_HeartlessTale.GI_HeartlessTale_C|GetThirdChoice (Variables|Default|GetCast%20To%20GI))
    (Input|EnableInput (Game|GetPlayerController 0))
    (bind _returnvalue (UserInterface|CreateWidget "/Game/UI/Blueprints/WBP_Interaction.WBP_Interaction_C"))
    (UserInterface|Viewport|AddtoViewport _returnvalue 0)
    (Default|ShowE _returnvalue)))

(event OnComponentEndOverlap(Box)
  (params (OverlappedComponent :type Primitive%20Component%20Object%20Reference) (OtherActor :type Actor%20Object%20Reference) (OtherComp :type Primitive%20Component%20Object%20Reference) (OtherBodyIndex :type Integer))
  ;[1 1 1] Zone dans laquelle linteraction est possible
  (if (Variables|/Game/Blueprints/GI_HeartlessTale.GI_HeartlessTale_C|GetThirdChoice (Variables|Default|GetCast%20To%20GI))
    (Input|DisableInput (Game|GetPlayerController 0))
    (Default|HideE (stale OnComponentBeginOverlap(Box) _returnvalue))))

(event Custom|PuppetVisible
  ;[1 1 1] Mesh résultant du choix
  (if (Variables|/Game/Blueprints/GI_HeartlessTale.GI_HeartlessTale_C|GetThirdChoice (Variables|Default|GetCast%20To%20GI))
    (AddComponent|AddPointLightComponent false (Math|Transform|MakeTransform "0,15.000000,50.000000" "0, 0, 0" "1.000000,1.000000,1.000000"))
    (if (Variables|/Game/Blueprints/GI_HeartlessTale.GI_HeartlessTale_C|Get3rdGoodChoice (Variables|Default|GetCast%20To%20GI))
      (AddComponent|AddStaticMeshComponent false (Math|Transform|MakeTransform "0, 0, 0" "0,165.000000,-60.000000" "4.000000,4.000000,4.000000"))
      (else
        (AddComponent|AddStaticMeshComponent false (Math|Transform|MakeTransform "0, 0, 0" "0,165.000000,-60.000000" "4.000000,4.000000,4.000000"))))))

(event EventBeginPlay
  (bind _asbp_third_person_character (Utilities|Casting|CastToBP_ThirdPersonCharacter (Game|Player|GetPlayerPawn 0)))
  (Variables|Default|SetCast%20To%20TPChara _asbp_third_person_character)
  (bind _asgi_heartless_tale (Utilities|Casting|CastToGI_HeartlessTale (Game|GetGameInstance)))
  (Variables|Default|SetCast%20To%20GI _asgi_heartless_tale)
  (CallFunction|PuppetVisible))

(event Input|ActionEvents|InputActionInteraction
  (params (Key :type Key%20Structure :default "None"))
  (bind _cast_to_tpchara (Variables|Default|GetCast%20To%20TPChara))
  ;[1 1 1] Interaction avec la fleur ou la poupée
  (:Pressed
    (if (Variables|Default|GetAlready%20Interacting)
      (Variables|Default|SetAlready%20Interacting false)
      (Default|UnlockInput _cast_to_tpchara)
      (Game|Player|SetViewTargetwithBlend (Game|GetPlayerController 0) (Game|Player|GetPlayerPawn 0) 0.5 "VTBlend_Linear" 0.0 false) ; Blend la caméra de ThirdPerson à celle du BP
      (Default|HideTextLabo (stale _returnvalue))
      (else
        (Variables|Default|SetAlready%20Interacting true)
        (Default|LockInput _cast_to_tpchara)
        (Game|Player|SetViewTargetwithBlend (Game|GetPlayerController 0) self 1.5 "VTBlend_Linear" 0.0 false) ; Blend la caméra de ThirdPerson à celle du BP
        (bind _returnvalue (UserInterface|CreateWidget "/Game/UI/Blueprints/WBP_LaboObjectsInteraction.WBP_LaboObjectsInteraction_C"))
        (UserInterface|Viewport|AddtoViewport _returnvalue 0)
        (Default|ShownTextLabo _returnvalue)
        (if (Variables|/Game/Blueprints/GI_HeartlessTale.GI_HeartlessTale_C|Get3rdGoodChoice (Variables|Default|GetCast%20To%20GI))
          (Default|TextLaboE _returnvalue "La poupée trouvée dans la Forêt des Myrrhades... Un souvenir efficace.")
          (else
            (Default|TextLaboE _returnvalue "Bêta conseille de cultiver cette fleur dans un endroit bien aéré... 
C'est le mieux qu'on puisse faire par ici.")))))))

(fn ConstructionScript)