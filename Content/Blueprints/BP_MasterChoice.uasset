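; BP_MasterChoice is an interactable actor that presents the player with a choice between a good option and a kill option.
; On Interact, it blends the player's camera from their current view to itself and displays a WBP_Choix1 widget.
; It binds to the widget's two choice dispatchers, and both outcomes currently just destroy the actor.
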(event Custom|Goodchoice
  (Actor|DestroyActor))

(event Custom|KillChoice
  (Actor|DestroyActor))

(event EventInteract
  (Utilities|FlowControl|Sequence
    (:then_0
      (Game|Player|SetViewTargetwithBlend (Game|GetPlayerController 0) self 2.0 "VTBlend_Linear" 0.0 false) ; Blend la caméra de ThirdPerson à celle du BP
    )
    (:then_1
      (bind _returnvalue (UserInterface|CreateWidget "/Game/UI/WBP_Choix1.WBP_Choix1_C")) ; Affiche le widget
      (bind _output_get (Variables|Default|SetUI_Choix _returnvalue))
      (EventDispatchers|BindEventtoOnGoodChoiceSelected _output_get (delegate Custom|Goodchoice))
      (EventDispatchers|BindEventtoOnKillChoiceSelected _output_get (delegate Custom|KillChoice))
      (UserInterface|Viewport|AddtoViewport _output_get 0))))

(fn ConstructionScript)