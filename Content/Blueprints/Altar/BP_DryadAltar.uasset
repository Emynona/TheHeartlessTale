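; Dryad altar that the player inspects to open the Myrrhade codex and, once the third choice is made, unlock the laboratory exit.
; An overlap box enables input and the prompt; interacting toggles player lock and a camera blend to the altar.
; With that choice set, it also destroys BP_Bêta's codex, spawns a highlight and updates the objective.
; On BeginPlay, GameInstance choice flags reveal the matching altar props.
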(event OnComponentBeginOverlap(Box)
  (params (OverlappedComponent :type Primitive%20Component%20Object%20Reference) (OtherActor :type Actor%20Object%20Reference) (OtherComp :type Primitive%20Component%20Object%20Reference) (OtherBodyIndex :type Integer) (bFromSweep :type Boolean) (SweepResult :type Hit%20Result%20Structure%20%28by%20ref%29))
  ;[1 1 1] Zone dans laquelle linteraction est possible
  (Input|EnableInput (Game|GetPlayerController 0))
  (bind _returnvalue (UserInterface|CreateWidget "/Game/UI/Blueprints/WBP_Interaction.WBP_Interaction_C"))
  (UserInterface|Viewport|AddtoViewport _returnvalue 0)
  (Default|ShowE _returnvalue))

(event OnComponentEndOverlap(Box)
  (params (OverlappedComponent :type Primitive%20Component%20Object%20Reference) (OtherActor :type Actor%20Object%20Reference) (OtherComp :type Primitive%20Component%20Object%20Reference) (OtherBodyIndex :type Integer))
  ;[1 1 1] Zone dans laquelle linteraction est possible
  (Input|DisableInput (Game|GetPlayerController 0))
  (Default|HideE (stale OnComponentBeginOverlap(Box) _returnvalue)))

(event Custom|ReturnButton
  (Variables|Default|SetAlready%20Interacting false)
  (Default|UnlockInput (Variables|Default|Getcast%20to%20third))
  (Game|Player|SetViewTargetwithBlend (Game|GetPlayerController 0) (Game|Player|GetPlayerPawn 0) 0.5 "VTBlend_Linear" 0.0 false) ; Blend la caméra de ThirdPerson à celle du BP
  (Variables|/Game/UI/Blueprints/WBP_CodexMyrrhade.WBP_CodexMyrrhade_C|SetHideParchment (stale Input|ActionEvents|InputActionInteraction _returnvalue) 0)
  (Default|ShowE (stale OnComponentBeginOverlap(Box) _returnvalue))
  (if (Variables|/Game/UI/Blueprints/WBP_Objectives.WBP_Objectives_C|GetIsHide (Variables|/Game/ThirdPerson/Blueprints/BP_ThirdPersonCharacter.BP_ThirdPersonCharacter_C|GetWBP_Objectives (Variables|Default|Getcast%20to%20third)))
    (Default|Show (Variables|/Game/ThirdPerson/Blueprints/BP_ThirdPersonCharacter.BP_ThirdPersonCharacter_C|GetWBP_Objectives (Variables|Default|Getcast%20to%20third)))))

(event Custom|ObjectCheck
  (Utilities|FlowControl|Sequence
    (:then_0
      (if (Variables|/Game/Blueprints/GI_HeartlessTale.GI_HeartlessTale_C|GetFirstChoice (Variables|Default|GetCast%20To%20GI))
        (Rendering|SetVisibility (Variables|Default|GetSM_TornCloth) true false)))
    (:then_1
      (if (Variables|/Game/Blueprints/GI_HeartlessTale.GI_HeartlessTale_C|GetSecondChoice (Variables|Default|GetCast%20To%20GI))
        (Rendering|SetVisibility (Variables|Default|GetCollar) true false)))
    (:then_2
      (if (Variables|/Game/Blueprints/GI_HeartlessTale.GI_HeartlessTale_C|GetThirdChoice (Variables|Default|GetCast%20To%20GI))
        (Rendering|SetVisibility (Variables|Default|GetSM_FlowerFrame) true false)))))

(event EventBeginPlay
  (bind _returnvalue (Actor|GetActorOfClass "/Game/Blueprints/BP_Bêta.BP_Bêta_C"))
  (Variables|Default|SetBP_Bêta _returnvalue)
  (bind _asgi_heartless_tale (Utilities|Casting|CastToGI_HeartlessTale (Game|GetGameInstance)))
  (Variables|Default|SetCast%20To%20GI _asgi_heartless_tale)
  (bind _asbp_third_person_character (Utilities|Casting|CastToBP_ThirdPersonCharacter (Game|GetPlayerCharacter 0)))
  (Variables|Default|Setcast%20to%20third _asbp_third_person_character)
  (CallFunction|ObjectCheck))

(event EventInteract
  ;[1 1 1] Line Trace Method
)

(event Input|ActionEvents|InputActionInteraction
  (params (Key :type Key%20Structure :default "None"))
  (bind _cast_to_third (Variables|Default|Getcast%20to%20third))
  (bind _cast_to_third_2 (Variables|Default|Getcast%20to%20third))
  (bind _wbp_objectives (Variables|/Game/ThirdPerson/Blueprints/BP_ThirdPersonCharacter.BP_ThirdPersonCharacter_C|GetWBP_Objectives _cast_to_third_2))
  (:Pressed
    (if (Variables|Default|GetAlready%20Interacting)
      (Variables|Default|SetAlready%20Interacting false)
      (Default|UnlockInput _cast_to_third)
      (Game|Player|SetViewTargetwithBlend (Game|GetPlayerController 0) (Game|Player|GetPlayerPawn 0) 0.5 "VTBlend_Linear" 0.0 false) ; Blend la caméra de ThirdPerson à celle du BP
      (Variables|/Game/UI/Blueprints/WBP_CodexMyrrhade.WBP_CodexMyrrhade_C|SetHideParchment (stale _returnvalue) 0)
      (Default|ShowE (stale OnComponentBeginOverlap(Box) _returnvalue))
      (if (Variables|/Game/UI/Blueprints/WBP_Objectives.WBP_Objectives_C|GetIsHide (Variables|/Game/ThirdPerson/Blueprints/BP_ThirdPersonCharacter.BP_ThirdPersonCharacter_C|GetWBP_Objectives (Variables|Default|Getcast%20to%20third)))
        (Default|Show _wbp_objectives))
      (else
        (Variables|Default|SetAlready%20Interacting true)
        (Default|LockInput _cast_to_third)
        (Game|Player|SetViewTargetwithBlend (Game|GetPlayerController 0) self 1.5 "VTBlend_Linear" 0.0 false) ; Blend la caméra de ThirdPerson à celle du BP
        (bind _returnvalue (UserInterface|CreateWidget "/Game/UI/Blueprints/WBP_CodexMyrrhade.WBP_CodexMyrrhade_C"))
        (UserInterface|Viewport|AddtoViewport _returnvalue 0)
        (Default|HideE (stale OnComponentBeginOverlap(Box) _returnvalue))
        (Utilities|FlowControl|Sequence
          (:then_0
            (if (not (Variables|/Game/UI/Blueprints/WBP_Objectives.WBP_Objectives_C|GetIsHide _wbp_objectives))
              (Default|Hide _wbp_objectives)))
          (:then_1
            (if (Variables|/Game/Blueprints/GI_HeartlessTale.GI_HeartlessTale_C|GetThirdChoice (Variables|Default|GetCast%20To%20GI))
              (Components|DestroyComponent (Variables|/Game/Blueprints/BP_Bêta.BP_Bêta_C|GetCodex (Variables|Default|GetBP_Bêta)))
              (Niagara|SpawnSystematLocation "/Game/Art/FX/Highlight/NS_HighlightLabo.NS_HighlightLabo" "1400.000000,-0.500000,1.000000")
              (Variables|/Game/Blueprints/GI_HeartlessTale.GI_HeartlessTale_C|SetUnlockEndDoor (Variables|Default|GetCast%20To%20GI) true)
              (Default|SetObjectif (Variables|/Game/ThirdPerson/Blueprints/BP_ThirdPersonCharacter.BP_ThirdPersonCharacter_C|GetWBP_Objectives (Variables|Default|Getcast%20to%20third)) "Sortir du laboratoire")
              (Default|AfterAltarQuest (Variables|Default|GetBP_Bêta)))))))))

(fn ConstructionScript)