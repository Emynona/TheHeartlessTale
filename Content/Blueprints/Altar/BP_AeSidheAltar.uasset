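; BP_AeSidheAltar is an interactable altar that opens the Aes Sidhe codex screen.
; BeginPlay caches references to the BP_Bêta actor, the GI_HeartlessTale game instance and the third-person player character, none of which are used elsewhere in this graph.
; Interact adds a WBP_CodexAesSidhe widget to the viewport and smoothly blends the player's view target to the altar itself.
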(event EventBeginPlay
  (bind _returnvalue (Actor|GetActorOfClass "/Game/Blueprints/BP_Bêta.BP_Bêta_C"))
  (Variables|Default|SetBP_Bêta _returnvalue)
  (bind _asgi_heartless_tale (Utilities|Casting|CastToGI_HeartlessTale (Game|GetGameInstance)))
  (Variables|Default|SetCast%20To%20GI _asgi_heartless_tale)
  (bind _asbp_third_person_character (Utilities|Casting|CastToBP_ThirdPersonCharacter (Game|GetPlayerCharacter 0)))
  (Variables|Default|Setcast%20to%20third _asbp_third_person_character))

(event EventInteract
  (bind _returnvalue (UserInterface|CreateWidget "/Game/UI/Blueprints/WBP_CodexAesSidhe.WBP_CodexAesSidhe_C"))
  (UserInterface|Viewport|AddtoViewport _returnvalue 0)
  (Game|Player|SetViewTargetwithBlend (Game|GetPlayerController 0) self 1.5 "VTBlend_Linear" 0.0 false) ; Blend la caméra de ThirdPerson à celle du BP
)

(fn ConstructionScript)