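; GI_HeartlessTale, apparently the game instance, records a LastPosition transform derived from the player's third-person character.
; LastPositionTransform finds the BP_ThirdPersonCharacter actor and reads its transform.
; It saves a location offset along the character's forward vector, with the same scale and the yaw manually rotated by a quarter turn.
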(fn LastPositionTransform
  (bind _returnvalue (Actor|GetActorOfClass "/Game/ThirdPerson/Blueprints/BP_ThirdPersonCharacter.BP_ThirdPersonCharacter_C"))
  (Variables|Default|SetLastPosition (Math|Transform|MakeTransform (+ (* (Math|Vector|GetForwardVector (Transformation|GetActorRotation _returnvalue)) 1e+02) (.Location (Math|Transform|BreakTransform (Transformation|GetActorTransform _returnvalue)))) (Math|Rotator|MakeRotator (.Roll (Math|Rotator|BreakRotator (.Rotation (Math|Transform|BreakTransform (Transformation|GetActorTransform _returnvalue))))) (.Pitch (Math|Rotator|BreakRotator (.Rotation (Math|Transform|BreakTransform (Transformation|GetActorTransform _returnvalue))))) (+ (.Yaw (Math|Rotator|BreakRotator (.Rotation (Math|Transform|BreakTransform (Transformation|GetActorTransform _returnvalue))))) 9e+01)) (.Scale (Math|Transform|BreakTransform (Transformation|GetActorTransform _returnvalue))))))