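; Menu book actor that shows a sequence of illustrated page spreads, then opens the laboratory level behind a loading widget.
; ChangeMaterial puts dynamic instances from the left and right material arrays on both page meshes and starts a dissolve timeline.
; That timeline plays forward, reverses, then calls ChangeMaterial again, looping until the array runs out.
; Separate events set and dissolve the opening illustration; a mesh-swapping variant is left disconnected.
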(event Custom|SetGameMode
  (bind _returnvalue (Game|GetPlayerController 0))
  ;[1 1 1] LE MIEN
  (Variables|/Script/Engine.PlayerController|SetbShowMouseCursor _returnvalue false)
  (Input|SetInputModeGameOnly _returnvalue))

(event Custom|StartDissolve
  (bind _mi_rightpage (Variables|Default|GetMI_RightPage))
  (bind _mi_leftpage (Variables|Default|GetMI_LeftPage))
  ;[1 1 1] LE MIEN
  (bind _dissolve (Timeline|Anim%20Dissolve PlayFromStart)
    (:Update
      (Utilities|IsValid _mi_rightpage
        (:Is%20Valid
          (Rendering|Material|SetScalarParameterValue _mi_rightpage "Dissolve" _dissolve :!class /Script/Engine.MaterialInstanceDynamic)
          (Utilities|IsValid _mi_leftpage
            (:Is%20Valid
              (Rendering|Material|SetScalarParameterValue _mi_leftpage "Dissolve" _dissolve :!class /Script/Engine.MaterialInstanceDynamic))))))
    (:Finished
      (if (Variables|Default|GetReversed)
        (CallFunction|ChangeMaterial)
        (else
          (Variables|Default|SetReversed true)
          (Timeline|Anim%20Dissolve ReverseFromEnd))))))

(event Custom|ChangeMaterial
  ;[1 1 1] LE MIEN
  (if (> (Variables|Default|GetMaterialToGet) (- (Utilities|Array|Length (Variables|Default|GetMI_Right)) 1))
    (bind _returnvalue (UserInterface|CreateWidget "/Game/UI/Blueprints/WBP_LoadingPhi.WBP_LoadingPhi_C"))
    (UserInterface|Viewport|AddtoViewport _returnvalue 0)
    (Game|OpenLevel(byName) "Lvl_Laboratory_Main")
    (CallFunction|SetGameMode)
    (else
      (Variables|Default|SetReversed false)
      (bind _returnvalue_2 (Rendering|Material|CreateDynamicMaterialInstance (Utilities|Array|Get(acopy) (Variables|Default|GetMI_Right) (Variables|Default|GetMaterialToGet)) "None" "None" :!class /Script/Engine.KismetMaterialLibrary))
      (bind _output_get (Variables|Default|SetMI_RightPage _returnvalue_2))
      (Rendering|Material|SetMaterial (Variables|Default|GetSM_PageMenuTestRight) 0 _output_get)
      (bind _returnvalue_3 (Rendering|Material|CreateDynamicMaterialInstance (Utilities|Array|Get(acopy) (Variables|Default|GetMI_Left) (Variables|Default|GetMaterialToGet)) "None" "None" :!class /Script/Engine.KismetMaterialLibrary))
      (bind _output_get_2 (Variables|Default|SetMI_LeftPage _returnvalue_3))
      (Rendering|Material|SetMaterial (Variables|Default|GetSM_PageMenuTestLeft) 0 _output_get_2)
      (Variables|Default|SetMaterialToGet (+ (Variables|Default|GetMaterialToGet) 1))
      (CallFunction|StartDissolve))))

(event Custom|ChangeStaticMesh
  ;[1 1 1] LE MIEN
)

(event Custom|EraseStartIllu
  ;[1 1 1] Illustration de début
  ;;[1 1 1] Do not forget to edit timeline duration in level bp if changed <3
  (bind _dissolve (Timeline|Timeline_0 ReverseFromEnd)
    (:Update
      (Rendering|Material|SetScalarParameterValue (stale Custom|CreateStartIllu _returnvalue) "Dissolve" _dissolve :!class /Script/Engine.MaterialInstanceDynamic))))

(event Custom|CreateStartIllu
  ;[1 1 1] Illustration de début
  (bind _returnvalue (Rendering|Material|CreateDynamicMaterialInstance "/Game/Art/Environment/CraftedRessources/DeskMenu/MI_PageMenu.MI_PageMenu" "None" "None" :!class /Script/Engine.KismetMaterialLibrary))
  (Rendering|Material|SetScalarParameterValue _returnvalue "Dissolve" 1.0 :!class /Script/Engine.MaterialInstanceDynamic)
  (Rendering|Material|SetMaterial (Variables|Default|GetSM_PageMenuTestRight) 0 _returnvalue))

(event Custom|First%20Dissolve
  ;[1 1 1] LE MIEN
  (Timeline|Blanc%20du%20début PlayFromStart))

(fn ConstructionScript)