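; BP_TreeChoice is a child choice Blueprint for what appears to be the game's first choice, at a tree.
; Interact runs the parent logic, then flags FirstChoice and CanTp as true on the GI_HeartlessTale game instance.
; KillChoice and Goodchoice both set 1stGoodChoice to false before calling their parent versions, reusing the cast result from Interact.
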(event EventBeginPlay)

(event Collision|EventActorBeginOverlap
  (params (OtherActor :type Actor%20Object%20Reference)))

(event EventTick
  (params (DeltaSeconds :type Float%20%28single-precision%29)))

(event EventInteract
  (|CallParentFunction) ; Play la logique du parent
  (bind _asgi_heartless_tale (Utilities|Casting|CastToGI_HeartlessTale (Game|GetGameInstance)))
  (Variables|/Game/Blueprints/GI_HeartlessTale.GI_HeartlessTale_C|SetFirstChoice _asgi_heartless_tale true)
  (Variables|/Game/Blueprints/GI_HeartlessTale.GI_HeartlessTale_C|SetCanTp? _asgi_heartless_tale true))

(event EventKillChoice
  (Variables|/Game/Blueprints/GI_HeartlessTale.GI_HeartlessTale_C|Set1stGoodChoice (stale EventInteract _asgi_heartless_tale) false)
  (|CallParentFunction))

(event EventGoodchoice
  (Variables|/Game/Blueprints/GI_HeartlessTale.GI_HeartlessTale_C|Set1stGoodChoice (stale EventInteract _asgi_heartless_tale) false)
  (|CallParentFunction))

(fn ConstructionScript
  (|CallParentFunction))