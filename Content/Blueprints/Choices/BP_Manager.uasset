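; BP_Manager runs an ordered quest of three choice objects, starting with the tree and dog, each paired with a wall.
; Init events sort objects and walls into parallel arrays by class, spawning a Niagara highlight at the tree.
; UpdateQuest updates the wall matching the chosen object, then moves the highlight to the next object using per-object offsets.
; Separate events destroy a given wall or show an image widget briefly.
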(event Custom|UpdateFXPosition
  (params (Choice%20Object :type BP%20Master%20Choice%20Object%20Reference%20%28by%20ref%29))
  ;[1 1 1] UpdateFXPosition. Récupère l'integer de l'objet dans le tableau pour faire spawn un FX à son emplacement avec un offset précis dans son vector3
  (Variables|Default|SetChoice%20Object Choice%20Object)
  (CallFunction|UpdateFX)
  (if (not (== (Utilities|Array|FindItem (Variables|Default|GetObjectChoice) (Variables|Default|GetChoice%20Object)) 0))
    (if (== (Utilities|Array|FindItem (Variables|Default|GetObjectChoice) (Variables|Default|GetChoice%20Object)) 1)
      (bind (_x _y _z) (CallFunction|MakeLocationOffset (Variables|Default|GetChoice%20Object)))
      (CallFunction|FX (Math|Vector|MakeVector (+ _x -125.0) (+ _y 0.0) (+ _z -3e+01)))
      (elif (== (Utilities|Array|FindItem (Variables|Default|GetObjectChoice) (Variables|Default|GetChoice%20Object)) 2)
        (bind (_x_2 _y_2 _z_2) (CallFunction|MakeLocationOffset (Variables|Default|GetChoice%20Object)))
        (CallFunction|FX (Math|Vector|MakeVector (+ _x_2 -6e+01) (+ _y_2 2e+01) (+ _z_2 -2e+01)))))))

(event Custom|UpdateQuest
  (params (ChoiceObject :type BP%20Master%20Choice%20Object%20Reference))
  (bind _objectchoice (Variables|Default|GetObjectChoice))
  (bind _returnvalue (Utilities|Array|FindItem _objectchoice ChoiceObject))
  ;[1 1 1] UpdateQuest. Permet de retirer les objets et les murs. Lance UpdateFX après.
  (Default|Updatevisual (Utilities|Array|Get(acopy) (Variables|Default|GetObjectWalls) _returnvalue))
  (CallFunction|UpdateFXPosition (Utilities|Array|Get(acopy) (Variables|Default|GetObjectChoice) (+ _returnvalue 1))))

(event Custom|IniatilizeObjects
  (params (NewItem :type BP%20Master%20Choice%20Object%20Reference%20%28by%20ref%29))
  (bind _returnvalue (Utilities|GetClass NewItem))
  ;[1 1 1] Place les objets dans l'ordre dans le tableau
  (if (== _returnvalue "/Game/Blueprints/Choices/BP_ChoiceTree.BP_ChoiceTree_C")
    (Utilities|Array|SetArrayElem (Variables|Default|GetObjectChoice) 0 NewItem true)
    (bind (_x _y _z) (CallFunction|MakeLocationOffset NewItem))
    (CallFunction|FX (Math|Vector|MakeVector (+ _x 1.5e+02) (+ _y 3e+02) (+ _z -1.5e+02)))
    (elif (== _returnvalue "/Game/Blueprints/Choices/BP_ChoiceDog.BP_ChoiceDog_C")
      (Utilities|Array|SetArrayElem (Variables|Default|GetObjectChoice) 1 NewItem true)
      (else
        (Utilities|Array|SetArrayElem (Variables|Default|GetObjectChoice) 2 NewItem true)))))

(event Custom|IniatilizeWalls
  (params (NewItem :type BP%20Wall%20Master%20Object%20Reference%20%28by%20ref%29))
  (bind _returnvalue (Utilities|GetClass NewItem))
  ;[1 1 1] Place les murs dans l'ordre dans le tableau
  (if (== _returnvalue "/Game/Blueprints/Choices/BP_WallVine.BP_WallVine_C")
    (Utilities|Array|SetArrayElem (Variables|Default|GetObjectWalls) 0 NewItem true)
    (elif (== _returnvalue "/Game/Blueprints/Choices/BP_WallCave.BP_WallCave_C")
      (Utilities|Array|SetArrayElem (Variables|Default|GetObjectWalls) 1 NewItem true)
      (else
        (Utilities|Array|SetArrayElem (Variables|Default|GetObjectWalls) 2 NewItem true)))))

(event Custom|DestroyWall
  (params (Target :type Actor%20Object%20Reference))
  (Actor|DestroyActor Target))

(event Custom|UpdateFX
  ;[1 1 1] Update FX. Remplace le FX de l'objet précédant par celui du nouvel objet
  (Components|DestroyComponent (Variables|Default|GetNiagara))
  (Variables|Default|SetNiagara 0))

(event Custom|UpdateImages
  (params (Class :type User%20Widget%20Class%20Reference))
  (bind _returnvalue (UserInterface|CreateWidget Class))
  (bind _output_get (Variables|Default|SetChoice%20Image _returnvalue))
  (UserInterface|Viewport|AddtoViewport _output_get 0)
  (Utilities|FlowControl|Delay 2.5)
  (Widget|RemovefromParent (Variables|Default|GetChoice%20Image)))

(fn ConstructionScript)

(fn FX
  (params (Location :type Vector))
  (bind _returnvalue (Niagara|SpawnSystematLocation "/Game/Art/FX/Highlight/NS_HighlightForest.NS_HighlightForest" Location "0, 0, 0" "1.000000,1.000000,1.000000" false))
  (Variables|Default|SetNiagara _returnvalue))

(fn MakeLocationOffset
  (params (Target :type Actor%20Object%20Reference))
  (bind _returnvalue (Transformation|GetActorLocation Target))
  (bind (_x _y _z) (Class|KismetMathLibrary|BreakVector3f _returnvalue))
  (return _x _y _z))