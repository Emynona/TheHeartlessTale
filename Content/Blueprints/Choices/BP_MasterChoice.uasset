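; Base choice actor that presents a good-or-kill decision with voiced dialogue.
; Interacting blends the camera to it and switches to UI-only input; CreateWidget binds a WBP_ChoiceMaster child to the character's Good or Kill, then destroys the actor.
; InitializeSound starts a sound array that Tick advances as each line ends, or the character's A press skips, calling PlayDialogue on the dialogue widget alongside.
; ChoiceDialogues briefly shows a given widget; DialogueOBJChoix is empty.
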(event Custom|ChoiceDialogues
  (params (Class :type User%20Widget%20Class%20Reference))
  (bind _returnvalue (UserInterface|CreateWidget Class))
  (bind _output_get (Variables|Default|SetChoiceDial _returnvalue))
  (UserInterface|Viewport|AddtoViewport _output_get 0)
  (Utilities|FlowControl|Delay 2.0)
  (Widget|RemovefromParent (Variables|Default|GetChoiceDial)))

(event Custom|InitializeSound
  (params (NewSound :type Array%20of%20Sound%20Base%20Object%20References))
  ;[1 1 1] Event Skip Audio
  (Variables|Default|SetNewSound NewSound)
  (CallFunction|StartAudio))

(event Custom|CreateWidget
  (params (Class :type User%20Widget%20Class%20Reference))
  ;[1 1 1] Create Child Widget Event
  (bind _returnvalue (UserInterface|CreateWidget Class)) ; Affiche le widget
  (bind _output_get (Variables|Default|SetUI_Choix _returnvalue))
  (bind _aswbp_choice_master (Utilities|Casting|CastToWBP_ChoiceMaster _output_get)) ; Cast to Master afin d'avoir les targets des "bind event good/bad"
  (EventDispatchers|BindEventtoOnGoodChoiceSelected _aswbp_choice_master (delegate Custom|Goodchoice))
  (EventDispatchers|BindEventtoOnKillChoiceSelected _aswbp_choice_master (delegate Custom|KillChoice))
  (UserInterface|Viewport|AddtoViewport _aswbp_choice_master 0))

(event Custom|Goodchoice
  ;[1 1 1] Create Child Widget Event
  ;;[1 1 1] Good Choice
  (Default|Good (Variables|Default|GetCastToThirdChara))
  (Actor|DestroyActor))

(event Custom|StartAudio
  ;[1 1 1] Event Skip Audio
  (Audio|Components|Audio|SetSound (Variables|Default|GetSound) (Utilities|Array|Get(acopy) (Variables|Default|GetNewSound) (Variables|Default|GetAudioLine))) ; Met à jours le "Sound" avec le nouveau du tableau
  (Audio|Components|Audio|Play (Variables|Default|GetSound) 0.0) ; Joue le son
  (Actor|Tick|SetActorTickEnabled true) ; Réactive l'event tick
)

(event Custom|DialogueOBJChoix
  (params (DialoguesLigne1 :type Text) (DialogueLigne2 :type Text)))

(event Custom|KillChoice
  ;[1 1 1] Create Child Widget Event
  ;;[1 1 1] Evil Choice
  (Default|Kill (Variables|Default|GetCastToThirdChara))
  (Actor|DestroyActor))

(event Custom|AisPressed
  (CallFunction|SkipAudio))

(event Custom|SkipAudio
  ;[1 1 1] Event Skip Audio
  (Actor|Tick|SetActorTickEnabled false) ; Désactive l'event tick pendant la logique qui suit
  (if (> (Variables|Default|GetAudioLine) (- (Utilities|Array|Length (Variables|Default|GetNewSound)) 1)) ; Vérifie s'il reste des sons dans le tableau
    (Variables|Default|SetAudioLine 0) ; Si non, remet à 0 AudioLine et vide le tableau NewSound
    (Utilities|Array|Clear (Variables|Default|GetNewSound))
    (else
      (Audio|Components|Audio|Stop (Variables|Default|GetSound)) ; Si oui, l'arrête
      (Variables|Default|SetAudioLine (+ (Variables|Default|GetAudioLine) 1)) ; +1 dans le tableau
      (Default|PlayDialogue (Variables|/Game/ThirdPerson/Blueprints/BP_ThirdPersonCharacter.BP_ThirdPersonCharacter_C|GetWBP%20Dialogues (Variables|Default|GetCastToThirdChara))) ; Custom event dans WBP Dialogue
      (Audio|Components|Audio|SetSound (Variables|Default|GetSound) (Utilities|Array|Get(acopy) (Variables|Default|GetNewSound) (Variables|Default|GetAudioLine))) ; Met à jours le "Sound" avec le nouveau du tableau
      (Audio|Components|Audio|Play (Variables|Default|GetSound) 0.0) ; Joue le son
      (Actor|Tick|SetActorTickEnabled true) ; Réactive l'event tick
    )))

(event EventBeginPlay
  (Default|IniatilizeObjects (Variables|Default|GetManager) self)
  (bind _asbp_third_person_character (Utilities|Casting|CastToBP_ThirdPersonCharacter (Game|GetPlayerCharacter 0)))
  (bind _output_get (Variables|Default|SetCastToThirdChara _asbp_third_person_character))
  (EventDispatchers|BindEventtoAPressed _output_get (delegate Custom|AisPressed))
  (bind _asgi_heartless_tale (Utilities|Casting|CastToGI_HeartlessTale (Game|GetGameInstance)))
  (Variables|Default|SetCastToGI _asgi_heartless_tale))

(event EventTick
  (params (DeltaSeconds :type Float%20%28single-precision%29))
  ;[1 1 1] Event Tick
  (if (> (Variables|Default|GetAudioLine) (- (Utilities|Array|Length (Variables|Default|GetNewSound)) 1)) ; Verifie s'il reste des sons dans le tableau
    (CallFunction|SkipAudio)
    (elif (not (Audio|Components|Audio|IsPlaying (Variables|Default|GetSound))) ; Vérifie si "Sound" est en train dêtre joué
      (Actor|Tick|SetActorTickEnabled false) ; Désactive le tick
      (Variables|Default|SetAudioLine (+ (Variables|Default|GetAudioLine) 1)) ; +1 dans le tableau
      (CallFunction|StartAudio) ; Relance "StartAudio" avec le nouvel integer (donc nouveau son)
      (Default|PlayDialogue (Variables|/Game/ThirdPerson/Blueprints/BP_ThirdPersonCharacter.BP_ThirdPersonCharacter_C|GetWBP%20Dialogues (Variables|Default|GetCastToThirdChara))) ; Relance "PlayDialogue" avec les nouvelles integer
    )))

(event EventInteract
  (bind _returnvalue (Game|GetPlayerController 0))
  (Game|Player|SetViewTargetwithBlend (Game|GetPlayerController 0) self 1.2 "VTBlend_Linear" 0.0 false) ; Blend la caméra de ThirdPerson à celle du BP
  (Variables|/Script/Engine.PlayerController|SetbShowMouseCursor _returnvalue false)
  (Input|SetInputModeUIOnly _returnvalue 0 "DoNotLock"))

(fn ConstructionScript)