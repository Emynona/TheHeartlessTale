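; BP_ChoiceDog is the interactable dog encounter, the player's second moral choice, built on a parent choice Blueprint.
; A box overlap toggles a text prompt; interacting hides it, shows French dialogue about sending the animal through the portal, creates the choice widget and sets GameInstance progress and teleport flags.
; Kill and good outcomes record the decision in the GameInstance, then share one sequence updating Manager images, quest and objective.
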(event OnComponentBeginOverlap(Box)
  (params (OverlappedComponent :type Primitive%20Component%20Object%20Reference) (OtherActor :type Actor%20Object%20Reference) (OtherComp :type Primitive%20Component%20Object%20Reference) (OtherBodyIndex :type Integer) (bFromSweep :type Boolean) (SweepResult :type Hit%20Result%20Structure%20%28by%20ref%29))
  (Rendering|SetVisibility (Variables|Default|GetTextRender) true false))

(event OnComponentEndOverlap(Box)
  (params (OverlappedComponent :type Primitive%20Component%20Object%20Reference) (OtherActor :type Actor%20Object%20Reference) (OtherComp :type Primitive%20Component%20Object%20Reference) (OtherBodyIndex :type Integer))
  (Rendering|SetVisibility (Variables|Default|GetTextRender) false false))

(event EventBeginPlay
  (|CallParentFunction))

(event EventInteract
  (bind _casttothirdchara (Variables|Default|GetCastToThirdChara))
  (bind _wbp_dialogues (Variables|/Game/ThirdPerson/Blueprints/BP_ThirdPersonCharacter.BP_ThirdPersonCharacter_C|GetWBP%20Dialogues _casttothirdchara))
  (|CallParentFunction)
  (Default|InitializeDialogue _wbp_dialogues (Utilities|Array|MakeArray "Que fait cet animal ici ? Laisse tomber, il a l'air appétissant et je meurs de faim," "envois le moi à travers le portail comme la Myrrhade !"))
  (UserInterface|Viewport|AddtoViewport _wbp_dialogues 0)
  (CallFunction|CreateWidget "/Game/UI/Blueprints/Choices/WBP_ChoiceDog.WBP_ChoiceDog_C")
  (Variables|/Game/Blueprints/GI_HeartlessTale.GI_HeartlessTale_C|SetSecondChoice (Variables|Default|GetCastToGI) true) ; Récupère la variable du GameInstance pour la set True
  (Variables|/Game/Blueprints/GI_HeartlessTale.GI_HeartlessTale_C|SetCanTp? (Variables|Default|GetCastToGI) true)
  (Rendering|SetVisibility (Variables|Default|GetTextRender) false false))

(event EventKillChoice
  (Variables|/Game/Blueprints/GI_HeartlessTale.GI_HeartlessTale_C|Set2ndGoodChoice (Variables|Default|GetCastToGI) false)
  (|CallParentFunction)
  (Utilities|FlowControl|Sequence
    (:then_0
      (Default|UpdateImages (Variables|Default|GetManager) "/Game/UI/Blueprints/WBP_PortalDog.WBP_PortalDog_C"))
    (:then_1
      (Default|UpdateQuest (Variables|Default|GetManager) self))
    (:then_2
      (Default|SetObjectif (Variables|/Game/ThirdPerson/Blueprints/BP_ThirdPersonCharacter.BP_ThirdPersonCharacter_C|GetWBP_Objectives (Variables|Default|GetCastToThirdChara)) "Découvrir ce qu'il est arrivé"))))

(event EventGoodchoice
  (Variables|/Game/Blueprints/GI_HeartlessTale.GI_HeartlessTale_C|Set2ndGoodChoice (Variables|Default|GetCastToGI) true)
  (|CallParentFunction)
  (Utilities|FlowControl|Sequence
    (:then_0
      (Default|UpdateImages (Variables|Default|GetManager) "/Game/UI/Blueprints/WBP_PortalDog.WBP_PortalDog_C"))
    (:then_1
      (Default|UpdateQuest (Variables|Default|GetManager) self))
    (:then_2
      (Default|SetObjectif (Variables|/Game/ThirdPerson/Blueprints/BP_ThirdPersonCharacter.BP_ThirdPersonCharacter_C|GetWBP_Objectives (Variables|Default|GetCastToThirdChara)) "Découvrir ce qu'il est arrivé"))))

(fn ConstructionScript
  (|CallParentFunction))