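; BP_ChoiceTree is a child choice object for the Chrysalis Tree, where the player faces the first moral choice about a human turning into a Myrrhade.
; Interacting plays two timed French dialogue pairs, then creates the WBP_ChoiceTree widget and flags FirstChoice in the game instance.
; KillChoice and Goodchoice record the outcome there, call parent logic, then both update the Manager's images and quest.
; A box overlap toggles a text prompt's visibility.
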(event OnComponentBeginOverlap(Box)
  (params (OverlappedComponent :type Primitive%20Component%20Object%20Reference) (OtherActor :type Actor%20Object%20Reference) (OtherComp :type Primitive%20Component%20Object%20Reference) (OtherBodyIndex :type Integer) (bFromSweep :type Boolean) (SweepResult :type Hit%20Result%20Structure%20%28by%20ref%29))
  (Rendering|SetVisibility (Variables|Default|GetTextRender) true false))

(event OnComponentEndOverlap(Box)
  (params (OverlappedComponent :type Primitive%20Component%20Object%20Reference) (OtherActor :type Actor%20Object%20Reference) (OtherComp :type Primitive%20Component%20Object%20Reference) (OtherBodyIndex :type Integer))
  (Rendering|SetVisibility (Variables|Default|GetTextRender) false false))

(event EventBeginPlay
  (|CallParentFunction))

(event EventInteract
  (|CallParentFunction) ; Play la logique du parent
  (CallFunction|DialogueOBJChoix "Il s'agit d'un Arbre Chrysalide, c'est ainsi que les Myrrhades naissent." "À l'intérieur se trouve l'un des ces . . . humains, qui est en train d'être métamorphosé en Myrrhade.  ")
  (Utilities|FlowControl|Delay 8.0)
  (CallFunction|DialogueOBJChoix "L’influence de l’Arbre Cœur est faible ici [...]" "c’est une occasion unique, ne te préoccupe pas de l'humain, il ne s'agit que d’une race inférieure de toute manière....")
  (Utilities|FlowControl|Delay 8.0)
  (CallFunction|CreateWidget "/Game/UI/Blueprints/Choices/WBP_ChoiceTree.WBP_ChoiceTree_C") ; Joue le custom event présent dans le parent pour choisir le widget
  (Variables|/Game/Blueprints/GI_HeartlessTale.GI_HeartlessTale_C|SetFirstChoice (Variables|Default|GetCastToGI) true))

(event EventKillChoice
  (Variables|/Game/Blueprints/GI_HeartlessTale.GI_HeartlessTale_C|Set1stGoodChoice (Variables|Default|GetCastToGI) false)
  (|CallParentFunction)
  (Utilities|FlowControl|Sequence
    (:then_0
      (Default|UpdateImages (Variables|Default|GetManager) "/Game/UI/Blueprints/WBP_DeadMyrrha.WBP_DeadMyrrha_C"))
    (:then_1
      (Default|UpdateQuest (Variables|Default|GetManager) self))))

(event EventGoodchoice
  (Variables|/Game/Blueprints/GI_HeartlessTale.GI_HeartlessTale_C|Set1stGoodChoice (Variables|Default|GetCastToGI) true)
  (|CallParentFunction)
  (Utilities|FlowControl|Sequence
    (:then_0
      (Default|UpdateImages (Variables|Default|GetManager) "/Game/UI/Blueprints/WBP_DeadMyrrha.WBP_DeadMyrrha_C"))
    (:then_1
      (Default|UpdateQuest (Variables|Default|GetManager) self))))

(fn ConstructionScript
  (|CallParentFunction))