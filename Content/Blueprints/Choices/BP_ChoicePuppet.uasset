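; Interactable puppet for the game's third choice, a child choice Blueprint where Bêta's French dialogue asks the player to let a fragile flower grow inside it.
; Interacting chains a fade, sounds, dialogue and the Roue timeline, then creates the choice widget and sets GameInstance choice and teleport flags.
; Both outcomes record good or bad, then share the return-to-laboratory objective, closing dialogue and quest update.
; A box overlap toggles the text prompt.
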(event OnComponentBeginOverlap(Box)
  (params (OverlappedComponent :type Primitive%20Component%20Object%20Reference) (OtherActor :type Actor%20Object%20Reference) (OtherComp :type Primitive%20Component%20Object%20Reference) (OtherBodyIndex :type Integer) (bFromSweep :type Boolean) (SweepResult :type Hit%20Result%20Structure%20%28by%20ref%29))
  (Rendering|SetVisibility (Variables|Default|GetTextRender) true false))

(event OnComponentEndOverlap(Box)
  (params (OverlappedComponent :type Primitive%20Component%20Object%20Reference) (OtherActor :type Actor%20Object%20Reference) (OtherComp :type Primitive%20Component%20Object%20Reference) (OtherBodyIndex :type Integer))
  (Rendering|SetVisibility (Variables|Default|GetTextRender) false false))

(event EventBeginPlay
  (|CallParentFunction))

(event EventInteract
  (bind _casttothirdchara (Variables|Default|GetCastToThirdChara))
  (bind _wbp_dialogues (Variables|/Game/ThirdPerson/Blueprints/BP_ThirdPersonCharacter.BP_ThirdPersonCharacter_C|GetWBP%20Dialogues _casttothirdchara))
  (|CallParentFunction) ; Play la logique du parent
  (Timeline|DialogueFade PlayFromStart
    (:Finished
      (CallFunction|InitializeSound (Utilities|Array|MakeArray "/Game/Sound/Bruitages/Enviro/Water_Cave_Clean.Water_Cave_Clean" "/Game/Sound/Bruitages/Enviro/Droplet_Long.Droplet_Long" "/Game/Sound/Bruitages/Enviro/Water_Cave_Clean.Water_Cave_Clean" "/Game/Sound/Bruitages/Enviro/Droplet_Long.Droplet_Long"))
      (Default|InitializeDialogue _wbp_dialogues (Utilities|Array|MakeArray "Humm, des Myrrhades ont dû attaquer cette caravane, il ne reste quasiment rien" "des Humains, tu dois être proche de l’Arbre Cœur." "Regarde cette fleur, je l’ai vue dans les recherches de Père." "" "Une fois à maturité, elle sert à créer une potion décuplant les facultés psychiques." "Elle me sera indispensable pour me permettre de me venger… euh retrouver père je veux dire" "Elle est très fragile, tu vas devoir la laisser pousser dans cette poupée, à moins que tu" "n’aies encore envie de t'encombrer de babioles appartenant aux humains."))
      (UserInterface|Viewport|AddtoViewport _wbp_dialogues 0)
      (Timeline|Roue PlayFromStart
        (:Finished
          (CallFunction|CreateWidget "/Game/UI/Blueprints/Choices/WBP_ChoicePuppet.WBP_ChoicePuppet_C")
          (Variables|/Game/Blueprints/GI_HeartlessTale.GI_HeartlessTale_C|SetThirdChoice (Variables|Default|GetCastToGI) true)
          (Variables|/Game/Blueprints/GI_HeartlessTale.GI_HeartlessTale_C|SetCanTp? (Variables|Default|GetCastToGI) true)
          (Rendering|SetVisibility (Variables|Default|GetTextRender) false false))))))

(event EventKillChoice
  (bind _casttothirdchara (Variables|Default|GetCastToThirdChara))
  (bind _wbp_dialogues (Variables|/Game/ThirdPerson/Blueprints/BP_ThirdPersonCharacter.BP_ThirdPersonCharacter_C|GetWBP%20Dialogues _casttothirdchara))
  (Variables|/Game/Blueprints/GI_HeartlessTale.GI_HeartlessTale_C|Set3rdGoodChoice (Variables|Default|GetCastToGI) false)
  (|CallParentFunction)
  (Default|SetObjectif (Variables|/Game/ThirdPerson/Blueprints/BP_ThirdPersonCharacter.BP_ThirdPersonCharacter_C|GetWBP_Objectives (Variables|Default|GetCastToThirdChara)) "Retourner au laboratoire")
  (Default|InitializeDialogue _wbp_dialogues (Utilities|Array|MakeArray "Excellent, avec cette potion il me sera facile de faire face à père." "Rentre au laboratoire, j’ai trouvé comment atteindre l’Arbre Cœur."))
  (UserInterface|Viewport|AddtoViewport _wbp_dialogues 0)
  (Default|UpdateQuest (Variables|Default|GetManager) self))

(event EventGoodchoice
  (bind _casttothirdchara (Variables|Default|GetCastToThirdChara))
  (bind _wbp_dialogues (Variables|/Game/ThirdPerson/Blueprints/BP_ThirdPersonCharacter.BP_ThirdPersonCharacter_C|GetWBP%20Dialogues _casttothirdchara))
  (Variables|/Game/Blueprints/GI_HeartlessTale.GI_HeartlessTale_C|Set3rdGoodChoice (Variables|Default|GetCastToGI) true)
  (|CallParentFunction)
  (Default|SetObjectif (Variables|/Game/ThirdPerson/Blueprints/BP_ThirdPersonCharacter.BP_ThirdPersonCharacter_C|GetWBP_Objectives (Variables|Default|GetCastToThirdChara)) "Retourner au laboratoire")
  (Default|InitializeDialogue _wbp_dialogues (Utilities|Array|MakeArray "Excellent, avec cette potion il me sera facile de faire face à père." "Rentre au laboratoire, j’ai trouvé comment atteindre l’Arbre Cœur."))
  (UserInterface|Viewport|AddtoViewport _wbp_dialogues 0)
  (Default|UpdateQuest (Variables|Default|GetManager) self))

(fn ConstructionScript
  (|CallParentFunction))