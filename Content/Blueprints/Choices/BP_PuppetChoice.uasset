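; BP_PuppetChoice is the puppet choice interactable, the third good-or-kill choice recorded in the Heartless Tale game instance.
; Interact runs the parent logic, creates the WBP_PuppetChoice widget, caches the game instance, and flags ThirdChoice and CanTp as true.
; Goodchoice and KillChoice set 3rdGoodChoice true or false on that cached instance, then defer to the parent, so both depend on Interact having run first.
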(event EventBeginPlay)

(event Collision|EventActorBeginOverlap
  (params (OtherActor :type Actor%20Object%20Reference)))

(event EventTick
  (params (DeltaSeconds :type Float%20%28single-precision%29)))

(event EventInteract
  (|CallParentFunction) ; Play la logique du parent
  (CallFunction|CreateWidget "/Game/UI/Blueprints/WBP_PuppetChoice.WBP_PuppetChoice_C")
  (bind _asgi_heartless_tale (Utilities|Casting|CastToGI_HeartlessTale (Game|GetGameInstance))) ; Récupère les variable 3rdGoodChoice + ThirdChoice
  (Variables|/Game/Blueprints/GI_HeartlessTale.GI_HeartlessTale_C|SetThirdChoice _asgi_heartless_tale true)
  (Variables|/Game/Blueprints/GI_HeartlessTale.GI_HeartlessTale_C|SetCanTp? _asgi_heartless_tale true))

(event EventKillChoice
  (Variables|/Game/Blueprints/GI_HeartlessTale.GI_HeartlessTale_C|Set3rdGoodChoice (stale EventInteract _asgi_heartless_tale) false)
  (|CallParentFunction))

(event EventGoodchoice
  (Variables|/Game/Blueprints/GI_HeartlessTale.GI_HeartlessTale_C|Set3rdGoodChoice (stale EventInteract _asgi_heartless_tale) true)
  (|CallParentFunction))

(fn ConstructionScript
  (|CallParentFunction))