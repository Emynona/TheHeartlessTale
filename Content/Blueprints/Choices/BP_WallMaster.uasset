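; BP_WallMaster is a wall actor that registers itself with a Manager on BeginPlay and can dissolve away before being destroyed.
; Its Updatevisual event swaps the static mesh slots to dynamic dissolve materials, using a rock set or a liana, root and leaf set depending on IsWall2Cave.
; A timeline for each variant drives the Dissolve scalar parameter, then asks the Manager to destroy the wall when it finishes.
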(event Custom|Updatevisual
  (bind _staticmesh (Variables|Default|GetStaticMesh))
  (bind _staticmesh_2 (Variables|Default|GetStaticMesh))
  (bind _staticmesh_3 (Variables|Default|GetStaticMesh))
  (if (Variables|Default|GetIsWall2Cave)
    ;[1 1 1] Wall2 dissolve material
    (bind _returnvalue (Rendering|Material|CreateDynamicMaterialInstance "/Game/Blueprints/Choices/MI_DissolveRockMedium.MI_DissolveRockMedium" "None" "None" :!class /Script/Engine.KismetMaterialLibrary))
    (Rendering|Material|SetMaterial _staticmesh_3 0 _returnvalue)
    (bind _returnvalue_2 (Rendering|Material|CreateDynamicMaterialInstance "/Game/Blueprints/Choices/MI_DissolveRockA.MI_DissolveRockA" "None" "None" :!class /Script/Engine.KismetMaterialLibrary))
    (Rendering|Material|SetMaterial _staticmesh_2 1 _returnvalue_2)
    (bind _returnvalue_3 (Rendering|Material|CreateDynamicMaterialInstance "/Game/Blueprints/Choices/MI_DissolveRockB.MI_DissolveRockB" "None" "None" :!class /Script/Engine.KismetMaterialLibrary))
    (Rendering|Material|SetMaterial _staticmesh 2 _returnvalue_3)
    (bind _newtrack_0 (Timeline|Timeline_1 PlayFromStart)
      (:Update
        (Rendering|Material|SetScalarParameterValue _returnvalue "Dissolve" _newtrack_0 :!class /Script/Engine.MaterialInstanceDynamic)
        (Rendering|Material|SetScalarParameterValue _returnvalue_2 "Dissolve" _newtrack_0 :!class /Script/Engine.MaterialInstanceDynamic)
        (Rendering|Material|SetScalarParameterValue _returnvalue_3 "Dissolve" _newtrack_0 :!class /Script/Engine.MaterialInstanceDynamic))
      (:Finished
        (Default|DestroyWall (Variables|Default|GetManager) self)))
    (else
      ;[1 1 1] Wall1 dissolve material
      (bind _returnvalue_4 (Rendering|Material|CreateDynamicMaterialInstance "/Game/Blueprints/Choices/MI_DissolveLianaA.MI_DissolveLianaA" "None" "None" :!class /Script/Engine.KismetMaterialLibrary))
      (Rendering|Material|SetMaterial _staticmesh_3 0 _returnvalue_4)
      (bind _returnvalue_5 (Rendering|Material|CreateDynamicMaterialInstance "/Game/Blueprints/Choices/MI_DissolveRootCurve.MI_DissolveRootCurve" "None" "None" :!class /Script/Engine.KismetMaterialLibrary))
      (Rendering|Material|SetMaterial _staticmesh_2 1 _returnvalue_5)
      (bind _returnvalue_6 (Rendering|Material|CreateDynamicMaterialInstance "/Game/Blueprints/Choices/MI_DissolveLeafD.MI_DissolveLeafD" "None" "None" :!class /Script/Engine.KismetMaterialLibrary))
      (Rendering|Material|SetMaterial _staticmesh 2 _returnvalue_6)
      (Rendering|Material|SetMaterial _staticmesh 3 _returnvalue_6)
      (bind _newtrack_0_2 (Timeline|Timeline_0 PlayFromStart)
        (:Update
          (Rendering|Material|SetScalarParameterValue _returnvalue_4 "Dissolve" _newtrack_0_2 :!class /Script/Engine.MaterialInstanceDynamic)
          (Rendering|Material|SetScalarParameterValue _returnvalue_5 "Dissolve" _newtrack_0_2 :!class /Script/Engine.MaterialInstanceDynamic)
          (Rendering|Material|SetScalarParameterValue _returnvalue_6 "Dissolve" _newtrack_0_2 :!class /Script/Engine.MaterialInstanceDynamic))
        (:Finished
          (Default|DestroyWall (Variables|Default|GetManager) self))))))

(event EventBeginPlay
  (Default|IniatilizeWalls (Variables|Default|GetManager) self))

(fn ConstructionScript)