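; BP_Dog is an interactable actor showing the outcome of the player's second choice: a resting dog or the remains of Bêta's meal.
; On BeginPlay it reads the choice flags from GI_HeartlessTale and adds the matching skeletal or static mesh.
; Once that choice is made, its box overlap toggles input and the interaction prompt.
; Interacting toggles the character's input lock, a camera blend to the actor and outcome-specific French text.
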(event OnComponentBeginOverlap(Box)
  (params (OverlappedComponent :type Primitive%20Component%20Object%20Reference) (OtherActor :type Actor%20Object%20Reference) (OtherComp :type Primitive%20Component%20Object%20Reference) (OtherBodyIndex :type Integer) (bFromSweep :type Boolean) (SweepResult :type Hit%20Result%20Structure%20%28by%20ref%29))
  ;[1 1 1] Zone dans laquelle linteraction est possible
  (if (Variables|/Game/Blueprints/GI_HeartlessTale.GI_HeartlessTale_C|GetSecondChoice (Variables|Default|GetCast%20To%20GI))
    (Input|EnableInput (Game|GetPlayerController 0))
    (bind _returnvalue (UserInterface|CreateWidget "/Game/UI/Blueprints/WBP_Interaction.WBP_Interaction_C"))
    (UserInterface|Viewport|AddtoViewport _returnvalue 0)
    (Default|ShowE _returnvalue)))

(event OnComponentEndOverlap(Box)
  (params (OverlappedComponent :type Primitive%20Component%20Object%20Reference) (OtherActor :type Actor%20Object%20Reference) (OtherComp :type Primitive%20Component%20Object%20Reference) (OtherBodyIndex :type Integer))
  ;[1 1 1] Zone dans laquelle linteraction est possible
  (if (Variables|/Game/Blueprints/GI_HeartlessTale.GI_HeartlessTale_C|GetSecondChoice (Variables|Default|GetCast%20To%20GI))
    (Input|DisableInput (Game|GetPlayerController 0))
    (Default|HideE (stale OnComponentBeginOverlap(Box) _returnvalue))))

(event Custom|DogVisible
  ;[1 1 1] Mesh résultant du choix
  (if (Variables|/Game/Blueprints/GI_HeartlessTale.GI_HeartlessTale_C|GetSecondChoice (Variables|Default|GetCast%20To%20GI))
    (if (Variables|/Game/Blueprints/GI_HeartlessTale.GI_HeartlessTale_C|Get2ndGoodChoice (Variables|Default|GetCast%20To%20GI))
      (AddComponent|AddSkeletalMeshComponent false (Math|Transform|MakeTransform "0.942665,6.116625,2.442876" "0, 0, 0" "1.300000,1.300000,1.300000"))
      (else
        (AddComponent|AddStaticMeshComponent false)))))

(event EventBeginPlay
  (bind _asbp_third_person_character (Utilities|Casting|CastToBP_ThirdPersonCharacter (Game|Player|GetPlayerPawn 0)))
  (Variables|Default|SetCast%20To%20TPChara _asbp_third_person_character)
  (bind _asgi_heartless_tale (Utilities|Casting|CastToGI_HeartlessTale (Game|GetGameInstance)))
  (Variables|Default|SetCast%20To%20GI _asgi_heartless_tale)
  (CallFunction|DogVisible))

(event Input|ActionEvents|InputActionInteraction
  (params (Key :type Key%20Structure :default "None"))
  (bind _cast_to_tpchara (Variables|Default|GetCast%20To%20TPChara))
  ;[1 1 1] Interaction avec le chien ou ses restes
  (:Pressed
    (if (Variables|Default|GetAlreadyInteracting)
      (Variables|Default|SetAlreadyInteracting false)
      (Default|UnlockInput _cast_to_tpchara)
      (Game|Player|SetViewTargetwithBlend (Game|GetPlayerController 0) (Game|Player|GetPlayerPawn 0) 0.5 "VTBlend_Linear" 0.0 false) ; Blend la caméra de ThirdPerson à celle du BP
      (Default|HideTextLabo (stale _returnvalue))
      (else
        (Variables|Default|SetAlreadyInteracting true)
        (Default|LockInput _cast_to_tpchara)
        (Game|Player|SetViewTargetwithBlend (Game|GetPlayerController 0) self 1.5 "VTBlend_Linear" 0.0 false) ; Blend la caméra de ThirdPerson à celle du BP
        (bind _returnvalue (UserInterface|CreateWidget "/Game/UI/Blueprints/WBP_LaboObjectsInteraction.WBP_LaboObjectsInteraction_C"))
        (UserInterface|Viewport|AddtoViewport _returnvalue 0)
        (Default|ShownTextLabo _returnvalue)
        (if (Variables|/Game/Blueprints/GI_HeartlessTale.GI_HeartlessTale_C|Get2ndGoodChoice (Variables|Default|GetCast%20To%20GI))
          (Default|TextLaboE _returnvalue "Ce chien se repose...Étrangement, Bêta s'est appliqué sur ses bandages...")
          (else
            (Default|TextLaboE _returnvalue "Il semblerait que ce soit tout ce qu'il reste du festin de Bêta... 
Puisse ce dernier avoir été satisfait...")))))))

(fn ConstructionScript)