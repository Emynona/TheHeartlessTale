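; PC_Phi, apparently a player controller, handles the pause menu input.
; MenuPause lazily creates WBP_PauseMenu, then branches on the paused state to remove it and unpause, or show it with cursor and UI-only input.
; The show branch never pauses the game itself.
; An unconnected interaction chain line-traces from the third-person character's camera and calls InteractMessage on BPI_Interact actors, but never runs.
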(event EventBeginPlay)

(event EventTick
  (params (DeltaSeconds :type Float%20%28single-precision%29)))

(event Input|ActionEvents|InputActionInteraction
  (params (Key :type Key%20Structure :default "None"))
  ;[1 1 1] Interface Interaction
)

(event Input|ActionEvents|InputActionMenuPause
  (params (Key :type Key%20Structure :default "None"))
  (bind _returnvalue (Game|GetPlayerController 0))
  (bind _returnvalue_2 (Game|GetPlayerController 0))
  ;[1 1 1] MenuPause
  (:Pressed
    (Utilities|IsValid (Variables|Default|GetPauseMenuRef)
      (:Is%20Valid
        _)
      (:Is%20Not%20Valid
        (bind _returnvalue_3 (UserInterface|CreateWidget "/Game/UI/WBP_PauseMenu.WBP_PauseMenu_C"))
        (Variables|Default|SetPauseMenuRef _returnvalue_3)))
    (if (Game|IsGamePaused) ; Vérifie si le jeu est déjà en pause
      (Game|SetGamePaused false) ; Met le jeu en pause
      (Widget|RemovefromParent (Variables|Default|GetPauseMenuRef)) ; Si oui, retire le widget
      (Variables|/Script/Engine.PlayerController|SetbShowMouseCursor _returnvalue_2 false) ; Retire le curseur de la souris
      (Input|SetInputModeGameOnly _returnvalue_2) ; Retire l'interactibilité du widget
      (else
        (UserInterface|Viewport|AddtoViewport (Variables|Default|GetPauseMenuRef) 0) ; Ajoute le widget à l'écran
        (Variables|/Script/Engine.PlayerController|SetbShowMouseCursor _returnvalue true) ; Affiche le curseur de la souris
        (Input|SetInputModeUIOnly _returnvalue 0 "DoNotLock") ; Rend le widget interactible
      ))))

(fn ConstructionScript)