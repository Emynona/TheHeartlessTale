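; BP_Door is a double door that opens near the player and serves as a level transition to Lvl_Forest.
; OpenBox overlaps play and reverse DoorTimeline, which yaws the left and right door meshes.
; TeleportBox overlap locks player input, plays an animated WBP_LoadingScreen, then opens the level after a short delay.
; Overlap handlers cast the fetched player rather than checking the overlapping actor, so any overlapping actor can trigger them.
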(event OnComponentEndOverlap(OpenBox)
  (params (OverlappedComponent :type Primitive%20Component%20Object%20Reference) (OtherActor :type Actor%20Object%20Reference) (OtherComp :type Primitive%20Component%20Object%20Reference) (OtherBodyIndex :type Integer))
  ;[1 1 1] DoorOpening
  (Utilities|Casting|CastToBP_ThirdPersonCharacter (Game|Player|GetPlayerPawn 0))
  (bind (_direction _doorrotaleft _doorrotaright) (Timeline|DoorTimeline Reverse)
    (:Update
      (Transformation|SetRelativeRotation (Variables|Default|GetSM_DoorLeft) (Math|Rotator|MakeRotator 0.0 0.0 _doorrotaleft) false false)
      (Transformation|SetRelativeRotation (Variables|Default|GetSM_DoorRight) (Math|Rotator|MakeRotator 0.0 0.0 _doorrotaright) false false))))

(event OnComponentBeginOverlap(TeleportBox)
  (params (OverlappedComponent :type Primitive%20Component%20Object%20Reference) (OtherActor :type Actor%20Object%20Reference) (OtherComp :type Primitive%20Component%20Object%20Reference) (OtherBodyIndex :type Integer) (bFromSweep :type Boolean) (SweepResult :type Hit%20Result%20Structure%20%28by%20ref%29))
  ;[1 1 1] Teleportation
  ;;[1 1 1] Récuperer l'event Lock du BP_ThirdPerson
  (bind _asbp_third_person_character (Utilities|Casting|CastToBP_ThirdPersonCharacter (Game|GetPlayerCharacter 0)))
  (Default|LockInput _asbp_third_person_character) ; Event permettant de bloquer les inputs de mouvement du joueur
  ;;[1 1 1] Affichage UI de chargement + Animation
  (bind _returnvalue (UserInterface|CreateWidget "/Game/UI/Blueprints/WBP_LoadingScreen.WBP_LoadingScreen_C")) ; Créé le Widget LoadingScreen
  (UserInterface|Viewport|AddtoViewport _returnvalue 0)
  (UserInterface|Animation|PlayAnimation _returnvalue 0 0.0 1 "Forward" 1.0 false) ; Lance l'animation de WBP_LoadingScreen
  (Utilities|FlowControl|Delay 2.5)
  (Game|OpenLevel(byName) "Lvl_Forest"))

(event OnComponentBeginOverlap(OpenBox)
  (params (OverlappedComponent :type Primitive%20Component%20Object%20Reference) (OtherActor :type Actor%20Object%20Reference) (OtherComp :type Primitive%20Component%20Object%20Reference) (OtherBodyIndex :type Integer) (bFromSweep :type Boolean) (SweepResult :type Hit%20Result%20Structure%20%28by%20ref%29))
  ;[1 1 1] DoorOpening
  (Utilities|Casting|CastToBP_ThirdPersonCharacter (Game|Player|GetPlayerPawn 0))
  (bind (_direction _doorrotaleft _doorrotaright) (Timeline|DoorTimeline Play)
    (:Update
      (Transformation|SetRelativeRotation (Variables|Default|GetSM_DoorLeft) (Math|Rotator|MakeRotator 0.0 0.0 _doorrotaleft) false false)
      (Transformation|SetRelativeRotation (Variables|Default|GetSM_DoorRight) (Math|Rotator|MakeRotator 0.0 0.0 _doorrotaright) false false))))

(fn ConstructionScript)