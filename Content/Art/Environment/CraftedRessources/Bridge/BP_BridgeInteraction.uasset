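; Interactable bridge Blueprint that lets the player inspect a destroyed bridge and read a French message saying it can no longer be crossed.
; A box overlap with the third-person character enables the actor's input and shows an E prompt widget, reversed on exit.
; The Interaction input toggles inspection: it locks character input, blends the view to this actor and displays the text widget, then unlocks, blends back and hides it.
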(event OnComponentBeginOverlap(Box)
  (params (OverlappedComponent :type Primitive%20Component%20Object%20Reference) (OtherActor :type Actor%20Object%20Reference) (OtherComp :type Primitive%20Component%20Object%20Reference) (OtherBodyIndex :type Integer) (bFromSweep :type Boolean) (SweepResult :type Hit%20Result%20Structure%20%28by%20ref%29))
  ;[1 1 1] Zone dans laquelle linteraction est possible
  (Utilities|Casting|CastToBP_ThirdPersonCharacter OtherActor)
  (Input|EnableInput (Game|GetPlayerController 0))
  (bind _returnvalue (UserInterface|CreateWidget "/Game/UI/Blueprints/WBP_Interaction.WBP_Interaction_C"))
  (UserInterface|Viewport|AddtoViewport _returnvalue 0)
  (Default|ShowE _returnvalue))

(event OnComponentEndOverlap(Box)
  (params (OverlappedComponent :type Primitive%20Component%20Object%20Reference) (OtherActor :type Actor%20Object%20Reference) (OtherComp :type Primitive%20Component%20Object%20Reference) (OtherBodyIndex :type Integer))
  ;[1 1 1] Zone dans laquelle linteraction est possible
  (Utilities|Casting|CastToBP_ThirdPersonCharacter OtherActor)
  (Input|DisableInput (Game|GetPlayerController 0))
  (Default|HideE (stale OnComponentBeginOverlap(Box) _returnvalue)))

(event EventBeginPlay
  (bind _asbp_third_person_character (Utilities|Casting|CastToBP_ThirdPersonCharacter (Game|Player|GetPlayerPawn 0)))
  (Variables|Default|SetCast%20To%20TPChara _asbp_third_person_character))

(event Input|ActionEvents|InputActionInteraction
  (params (Key :type Key%20Structure :default "None"))
  (bind _cast_to_tpchara (Variables|Default|GetCast%20To%20TPChara))
  ;[1 1 1] Interaction avec la fleur ou la poupée
  (:Pressed
    (if (Variables|Default|GetAlready%20Interacting)
      (Variables|Default|SetAlready%20Interacting false)
      (Default|UnlockInput _cast_to_tpchara)
      (Game|Player|SetViewTargetwithBlend (Game|GetPlayerController 0) (Game|Player|GetPlayerPawn 0) 0.5 "VTBlend_Linear" 0.0 false) ; Blend la caméra de ThirdPerson à celle du BP
      (Default|HideTextLabo (stale _returnvalue))
      (else
        (Variables|Default|SetAlready%20Interacting true)
        (Default|LockInput _cast_to_tpchara)
        (Game|Player|SetViewTargetwithBlend (Game|GetPlayerController 0) self 1.5 "VTBlend_Linear" 0.0 false) ; Blend la caméra de ThirdPerson à celle du BP
        (bind _returnvalue (UserInterface|CreateWidget "/Game/UI/Blueprints/WBP_LaboObjectsInteraction.WBP_LaboObjectsInteraction_C"))
        (UserInterface|Viewport|AddtoViewport _returnvalue 0)
        (Default|ShownTextLabo _returnvalue)
        (Default|TextLaboE _returnvalue "Ce pont ne pourra plus être traversé... 
Il a été violemment détruit.")))))

(fn ConstructionScript)