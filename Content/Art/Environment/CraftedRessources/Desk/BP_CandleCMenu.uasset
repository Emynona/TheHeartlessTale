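; Candle Blueprint for a desk prop, apparently a menu variant, with a point light.
; The construction script calls SetLightIntensity, which applies the Intensity variable to the light.
; BeginPlay is empty, and the graph's randomized base intensity and timeline-driven flicker logic are disconnected, so they never run and the light stays steady.
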(event Custom|SetLightIntensity
  (Rendering|Components|Light|SetIntensity (Variables|Default|GetPointLight) (Variables|Default|GetIntensity)))

(event EventBeginPlay)

(fn ConstructionScript
  (CallFunction|SetLightIntensity))