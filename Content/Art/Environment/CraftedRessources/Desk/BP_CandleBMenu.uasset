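; Candle prop, apparently for the menu by its name, with a flickering point light.
; BeginPlay starts a timeline at a random offset so copies do not flicker in sync.
; Its Flick track switches each update between base intensity and a random value between IntensityFlick and Intensity.
; The construction script applies the base intensity; random on/off and random base-intensity logic is left disconnected.
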(event Custom|SetLightIntensity
  (Rendering|Components|Light|SetIntensity (Variables|Default|GetPointLight) (Variables|Default|GetIntensity)))

(event EventBeginPlay
  (bind _intensity (Variables|Default|GetIntensity))
  (Utilities|FlowControl|Sequence ; SetStartTimeTL
    (:then_0
      (bind _flick (Timeline|Timeline_0 SetNewTime)
        (:Update
          ;[1 1 1] SetValues
          (Rendering|Components|Light|SetIntensity (Variables|Default|GetPointLight) (Math|Float|SelectFloat _intensity (Math|Random|RandomFloatinRange (Variables|Default|GetIntensityFlick) _intensity) (== _flick 0.0))))))
    (:then_1
      (Timeline|Timeline_0 Play))))

(fn ConstructionScript
  (CallFunction|SetLightIntensity))