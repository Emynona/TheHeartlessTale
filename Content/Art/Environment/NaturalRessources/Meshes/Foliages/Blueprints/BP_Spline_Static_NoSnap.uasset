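; Construction-script spline builder, labelled for mine walls and rails, that lays repeated meshes along every spline component under the root.
; It chains spline mesh segments sized from each mesh's Y bounds, with an optional second mesh and tangents clamped to segment length.
; An optional pass then spaces child actors along the last spline processed.
; A line-trace floor-snap function exists but is never run.
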(event Custom|Stem
  ;[1 1 1] MineWallAndRails
  ;;[1 1 1] All Spline are now the value "as spline component"
  (for _array_element (Components|GetChildrenComponents (Variables|Default|GetDefaultSceneRoot) false) ; Array obtenu = nombre delements sous default scene root
    (bind _asspline_component (Utilities|Casting|CastToSplineComponent _array_element))
    (Variables|Default|SetAs%20Spline%20Component _asspline_component)
    ;;[1 1 1] Splines
    (for _index (range 0 (Math|Float|Truncate (/ (Spline|GetSplineLength (Variables|Default|GetAs%20Spline%20Component)) (Variables|Default|GetSmallerSize))))
      (CallFunction|AddSpline _index (Variables|Default|GetMesh%20Axis%20Along%20Spline%201) (Variables|Default|GetMesh1) (Variables|Default|GetRelative%20Transform%20Location%201) (Variables|Default|GetMeshSize1))
      (if (Variables|Default|GetUseMesh2)
        (CallFunction|AddSpline _index (Variables|Default|GetMesh%20Axis%20Along%20Spline%202) (Variables|Default|GetMesh2) (Variables|Default|GetRelative%20Transform%20Location%202) (Variables|Default|GetMeshSize2))))))

(event Custom|CompareAB
  (bind _meshsize1 (Variables|Default|GetMeshSize1))
  (bind _meshsize2 (Variables|Default|GetMeshSize2))
  ;[1 1 1] MineWallAndRails
  ;;[1 1 1] Mesh automatically placed and always the same size along spline
  (if (>= _meshsize1 _meshsize2) ; MustKeepTheSmallerSizeMesh (Or it will cut before the end)
    (Variables|Default|SetSmallerSize _meshsize2)
    (else
      (Variables|Default|SetSmallerSize _meshsize1))))

(event Custom|Leaf
  (bind _bpelementdistance (Variables|Default|GetBPElementDistance))
  (bind _as_spline_component (Variables|Default|GetAs%20Spline%20Component))
  ;[1 1 1] AddBPElementAlongSpline
  (if (Variables|Default|GetUseSecondElement)
    (for _index (range 0 (/ (stale Custom|Stem _index) (Math|Float|Truncate _bpelementdistance)))
      (CallFunction|AddBP (Spline|GetLocationatDistanceAlongSpline _as_spline_component (* (* _index (Variables|Default|GetSmallerSize)) _bpelementdistance) "World") (Math|Rotator|MakeRotfromX (Spline|GetTangentatDistanceAlongSpline _as_spline_component (* (* _index (Variables|Default|GetSmallerSize)) _bpelementdistance) "Local"))))))

(fn ConstructionScript
  (bind _mesh1 (Variables|Default|GetMesh1))
  (bind _mesh2 (Variables|Default|GetMesh2))
  (bind _returnvalue (StaticMesh|GetBoundingBox _mesh2))
  (bind _returnvalue_2 (StaticMesh|GetBoundingBox _mesh1))
  (bind (_min _max) (Utilities|Struct|BreakBox _returnvalue_2))
  (bind (_min_2 _max_2) (Utilities|Struct|BreakBox _returnvalue))
  (CallFunction|CompareAB)
  ;[1 1 1] AutoMeshSize
  (Variables|Default|SetMeshSize1 (Math|Vector|VectorLength (Math|Vector|MakeVector 0.0 (.Y (Math|Vector|BreakVector (- _max _min))) 0.0)))
  (Variables|Default|SetMeshSize2 (Math|Vector|VectorLength (Math|Vector|MakeVector 0.0 (.Y (Math|Vector|BreakVector (- _max_2 _min_2))) 0.0)))
  (CallFunction|Stem)
  (CallFunction|Leaf))

(fn SplineSnaptoSurface
  (params (PointIndex :type Integer) (PointIndex1 :type Integer))
  (bind _as_spline_component (Variables|Default|GetAs%20Spline%20Component))
  (bind _returnvalue (Spline|GetLocationatSplinePoint _as_spline_component PointIndex1 "World"))
  ;[1 1 1] Snap To Floor
  (bind _outhit (Collision|LineTraceByChannel (* _returnvalue "1.000000,1.000000,100.000000") (* _returnvalue "1.000000,1.000000, 0") "TraceTypeQuery1" false 0 "ForDuration"))
  (Spline|SetLocationatSplinePoint _as_spline_component PointIndex (.ImpactPoint (Collision|BreakHitResult _outhit)) "World" true))

(fn AddSpline
  (params (LastIndex :type Integer) (InForwardAxis :type ESplineMeshAxis%20Enum :default "X") (NewMesh :type Static%20Mesh%20Object%20Reference) (Relative%20Transform%20Location :type Vector) (ObjectSize :type Float%20%28double-precision%29))
  (bind _returnvalue (Math|Float|Truncate ObjectSize))
  (bind _returnvalue_2 (+ LastIndex 1))
  (bind _as_spline_component (Variables|Default|GetAs%20Spline%20Component))
  (bind _returnvalue_3 (* _returnvalue_2 _returnvalue))
  (bind _returnvalue_4 (* LastIndex _returnvalue))
  (bind _returnvalue_5 (Math|Conversions|ToFloat(Integer) _returnvalue_4))
  (bind _returnvalue_6 (Math|Conversions|ToFloat(Integer) _returnvalue_3))
  ;[1 1 1] AddSpline
  (bind _returnvalue_7 (AddComponent|AddSplineMeshComponent false (Math|Transform|MakeTransform Relative%20Transform%20Location "0, 0, 0" "1.000000,1.000000,1.000000"))) ; Spline
  (SplineMesh|SetForwardAxis _returnvalue_7 InForwardAxis true) ; Mesh Follow Spline Axis
  (Components|StaticMesh|SetStaticMesh _returnvalue_7 NewMesh)
  (Collision|SetCollisionEnabled _returnvalue_7 "QueryAndPhysics") ; Collisions
  (SplineMesh|SetStartandEnd _returnvalue_7 (Spline|GetLocationatDistanceAlongSpline _as_spline_component _returnvalue_5 "Local") (Math|Vector|ClampVectorSize (Spline|GetTangentatDistanceAlongSpline _as_spline_component _returnvalue_5 "Local") 0.0 ObjectSize) (Spline|GetLocationatDistanceAlongSpline _as_spline_component _returnvalue_6 "Local") (Math|Vector|ClampVectorSize (Spline|GetTangentatDistanceAlongSpline _as_spline_component _returnvalue_6 "Local") 0.0 ObjectSize) true :!class /Script/Engine.SplineMeshComponent))

(fn AddBP
  (params (NewLocation :type Vector) (NewRotation :type Rotator))
  ;[1 1 1] AddBP
  (bind _returnvalue (AddComponent|AddChildActorComponent true))
  (Transformation|AttachComponentToComponent _returnvalue (Variables|Default|GetAs%20Spline%20Component) "None" "KeepRelative" "KeepRelative" "KeepRelative" true)
  (Transformation|SetWorldLocation _returnvalue NewLocation false false)
  (Transformation|SetRelativeRotation _returnvalue NewRotation false false))