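; Procedural foliage Blueprint that builds stems with leaves or other attachments along splines in the construction script.
; Stem loops over child splines, trace-snaps points to surfaces and lays one or two layers of spline meshes, auto-sized from mesh bounds, with progressive taper and roll.
; Leaf then places optional child actors and static meshes along the last processed spline, using randomized spacing, progressive scaling and random roll on the meshes.
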(event Custom|Stem
  ;[1 1 1] All Spline are now the value "as spline component"
  (for _array_element (Components|GetChildrenComponents (Variables|Default|GetDefaultSceneRoot) false) ; Array obtenu = nombre delements sous default scene root
    (bind _asspline_component (Utilities|Casting|CastToSplineComponent _array_element))
    (Variables|Default|SetAs%20Spline%20Component _asspline_component)
    (Utilities|FlowControl|Sequence
      (:then_0
        ;[1 1 1] Spline1
        (for _index (range 0 (Math|Float|Truncate (/ (Spline|GetSplineLength (Variables|Default|GetAs%20Spline%20Component)) (Variables|Default|GetMeshSize1))))
          (CallFunction|SplineSnaptoSurface _index _index)
          (CallFunction|AddSpline _index (Variables|Default|GetMesh%20Axis%20Along%20Spline%201) (Variables|Default|GetMesh1) (Variables|Default|GetRelative%20Transform%20Location%201) (Variables|Default|GetMeshSize1) (Variables|Default|GetMesh1Material))))
      (:then_1
        ;[1 1 1] Spline2
        (if (Variables|Default|GetUseMesh2)
          (Variables|Default|SetSplineScale 1.0)
          (for _index_2 (range 0 (Math|Float|Truncate (/ (Spline|GetSplineLength (Variables|Default|GetAs%20Spline%20Component)) (Variables|Default|GetMeshSize2))))
            (CallFunction|SplineSnaptoSurface _index_2 _index_2)
            (CallFunction|AddSpline _index_2 (Variables|Default|GetMesh%20Axis%20Along%20Spline%202) (Variables|Default|GetMesh2) (Variables|Default|GetRelative%20Transform%20Location%202) (Variables|Default|GetMeshSize2) (Variables|Default|GetMesh2Material))))))))

(event Custom|CompareAB
  (bind _meshsize2 (Variables|Default|GetMeshSize2))
  (bind _meshsize1 (Variables|Default|GetMeshSize1))
  ;[1 1 1] Mesh automatically placed and always the same size along spline
  (if (>= _meshsize1 _meshsize2) ; MustKeepTheSmallerSizeMesh (Or it will cut before the end)
    (Variables|Default|SetSmallerSize _meshsize2)
    (else
      (Variables|Default|SetSmallerSize _meshsize1))))

(event Custom|Leaf
  (bind _returnvalue (Math|Random|RandomFloatinRange 1.0 1.5))
  (bind _relative_transform_location_1 (Variables|Default|GetRelative%20Transform%20Location%201))
  (bind _actorspacing (Variables|Default|GetActorSpacing))
  (bind _as_spline_component (Variables|Default|GetAs%20Spline%20Component))
  (bind _returnvalue_2 (* _actorspacing _returnvalue))
  ;[1 1 1] AddActorElementAlongSpline
  (for _index (range 0 (Math|Float|Truncate (/ (Spline|GetSplineLength (Variables|Default|GetAs%20Spline%20Component)) _returnvalue_2)))
    ;;[1 1 1] Reduce Scale at each loop
    (Variables|Default|SetReducedActorScale (* (Variables|Default|GetReducedActorScale) (Variables|Default|GetActorSizeDistance)))
    (Utilities|FlowControl|Sequence
      (:then_0
        (CallFunction|AddChildActor _relative_transform_location_1 (Spline|GetLocationatDistanceAlongSpline _as_spline_component (* _index _returnvalue_2) "World") (Math|Conversions|RotationFromXVector (Spline|GetTangentatDistanceAlongSpline _as_spline_component (* _index _returnvalue_2) "Local")) (Math|Conversions|ToVector(Float) (* (Variables|Default|GetChildActorScale) (Variables|Default|GetReducedActorScale)))))
      (:then_1
        (CallFunction|AddStaticMesh _relative_transform_location_1 (Spline|GetLocationatDistanceAlongSpline _as_spline_component (* _index _returnvalue_2) "World") (Math|Rotator|MakeRotator (.Roll (Math|Rotator|BreakRotator (Math|Rotator|CombineRotators (Math|Rotator|MakeRotfromX (Spline|GetTangentatDistanceAlongSpline _as_spline_component (* _index _returnvalue_2) "Local")) (Math|Random|RandomRotator true)))) 0.0 0.0) (Math|Conversions|ToVector(Float) (* (Variables|Default|GetReducedActorScale) (Variables|Default|GetStaticMeshScale))))))))

(fn ConstructionScript
  (bind _mesh1 (Variables|Default|GetMesh1))
  (bind _mesh2 (Variables|Default|GetMesh2))
  (bind _returnvalue (StaticMesh|GetBoundingBox _mesh2))
  (bind _returnvalue_2 (StaticMesh|GetBoundingBox _mesh1))
  (bind (_min _max) (Utilities|Struct|BreakBox _returnvalue_2))
  (bind (_min_2 _max_2) (Utilities|Struct|BreakBox _returnvalue))
  ;[1 1 1] Reset variables
  (Variables|Default|SetSplineScale (* (Variables|Default|GetSplineScale) (Variables|Default|GetAdjustEndScale)))
  (Variables|Default|SetReducedActorScale 1.0)
  (Variables|Default|SetSplineRoll 1.0)
  ;[1 1 1] AutoMeshSize
  (Variables|Default|SetMeshSize1 (Math|Vector|VectorLength (Math|Vector|MakeVector 0.0 (.Y (Math|Vector|BreakVector (- _max _min))) 0.0)))
  (if (Variables|Default|GetUseMesh2)
    (Variables|Default|SetMeshSize2 (Math|Vector|VectorLength (Math|Vector|MakeVector 0.0 (.Y (Math|Vector|BreakVector (- _max_2 _min_2))) 0.0)))
    (else
      (Variables|Default|SetSmallerSize (Variables|Default|GetMeshSize1))))
  (CallFunction|CompareAB)
  (CallFunction|Stem)
  (CallFunction|Leaf))

(fn SplineSnaptoSurface
  (params (PointIndex :type Integer) (PointIndex1 :type Integer))
  (bind _as_spline_component (Variables|Default|GetAs%20Spline%20Component))
  (bind _returnvalue (Spline|GetLocationatSplinePoint _as_spline_component PointIndex1 "World"))
  ;[1 1 1] Snap To Floor
  (bind _outhit (Collision|LineTraceByChannel (* _returnvalue "1.000000,1.000000,100.000000") (* _returnvalue "1.000000,1.000000,0.000000") "TraceTypeQuery1" false 0 "None"))
  (Spline|SetLocationatSplinePoint _as_spline_component PointIndex (.ImpactPoint (Collision|BreakHitResult _outhit)) "World" true))

(fn AddSpline
  (params (LastIndex :type Integer) (InForwardAxis :type ESplineMeshAxis%20Enum :default "X") (NewMesh :type Static%20Mesh%20Object%20Reference) (Relative%20Transform%20Location :type Vector) (ObjectSize :type Float%20%28double-precision%29) (Material :type Material%20Interface%20Object%20Reference))
  (bind _returnvalue (Math|Float|Truncate ObjectSize))
  (bind _returnvalue_2 (+ LastIndex 1))
  (bind _as_spline_component (Variables|Default|GetAs%20Spline%20Component))
  (bind _returnvalue_3 (* _returnvalue_2 _returnvalue))
  (bind _returnvalue_4 (* LastIndex _returnvalue))
  (bind _returnvalue_5 (Math|Conversions|ToFloat(Integer) _returnvalue_4))
  (bind _returnvalue_6 (Math|Conversions|ToFloat(Integer) _returnvalue_3))
  ;[1 1 1] AddSpline
  (bind _returnvalue_7 (AddComponent|AddSplineMeshComponent false (Math|Transform|MakeTransform Relative%20Transform%20Location "0, 0, 0" "1.000000,1.000000,1.000000"))) ; Spline
  (Rendering|Material|SetMaterial _returnvalue_7 0 Material)
  (SplineMesh|SetForwardAxis _returnvalue_7 InForwardAxis true) ; Mesh Follow Spline Axis
  (Components|StaticMesh|SetStaticMesh _returnvalue_7 NewMesh)
  (if (Variables|Default|GetCollision)
    (Collision|SetCollisionEnabled _returnvalue_7 "QueryAndPhysics") ; Collisions
  )
  (CallFunction|MeshScaleSpline _returnvalue_7 ObjectSize)
  (CallFunction|MeshRollSpline _returnvalue_7 ObjectSize)
  (SplineMesh|SetStartandEnd _returnvalue_7 (Spline|GetLocationatDistanceAlongSpline _as_spline_component _returnvalue_5 "Local") (Math|Vector|ClampVectorSize (Spline|GetTangentatDistanceAlongSpline _as_spline_component _returnvalue_5 "Local") 0.0 ObjectSize) (Spline|GetLocationatDistanceAlongSpline _as_spline_component _returnvalue_6 "Local") (Math|Vector|ClampVectorSize (Spline|GetTangentatDistanceAlongSpline _as_spline_component _returnvalue_6 "Local") 0.0 ObjectSize) true :!class /Script/Engine.SplineMeshComponent))

(fn AddChildActor
  (params (RelativeLocation :type Vector) (Location :type Vector) (Rotation :type Rotator) (Scale :type Vector))
  (bind (_roll _pitch _yaw) (Math|Rotator|BreakRotator Rotation))
  (if (Variables|Default|GetUseChildActor)
    ;[1 1 1] AddWhateverChildActor
    (bind _returnvalue (AddComponent|AddChildActorComponent true (Math|Transform|MakeTransform "0, 0, 0" "0, 0, 0" (Math|Conversions|ToVector(Float) (Variables|Default|GetChildActorScale)))))
    (ChildActorComponent|SetChildActorClass _returnvalue (Variables|Default|GetChildActor))
    (Transformation|AttachComponentToComponent _returnvalue (Variables|Default|GetAs%20Spline%20Component) "None" "KeepRelative" "KeepRelative" "KeepRelative" true)
    (Transformation|SetWorldLocation _returnvalue (+ RelativeLocation Location) false false)
    (Transformation|SetRelativeRotation _returnvalue (Math|Rotator|MakeRotator 0.0 _pitch _yaw) false false)
    (Transformation|SetRelativeScale3D _returnvalue Scale)))

(fn MeshScaleSpline
  (params (SplineMeshComponent :type Spline%20Mesh%20Component%20Object%20Reference) (MeshSize :type Float%20%28double-precision%29))
  (Variables|Default|SetMeshStartScale (Variables|Default|GetMeshStartScale))
  ;[1 1 1] ScaleAlongSpline
  (SplineMesh|SetStartScale SplineMeshComponent (Math|Vector2D|MakeVector2D (* (Variables|Default|GetSplineScale) (Variables|Default|GetMeshStartScale)) (* (Variables|Default|GetSplineScale) (Variables|Default|GetMeshStartScale))) true :!class /Script/Engine.SplineMeshComponent)
  (bind _output_get (Variables|Default|SetSplineScale (- (Variables|Default|GetSplineScale) (/ 1.0 (/ (Spline|GetSplineLength (Variables|Default|GetAs%20Spline%20Component)) MeshSize)))))
  (SplineMesh|SetEndScale SplineMeshComponent (Math|Vector2D|MakeVector2D (* _output_get (Variables|Default|GetMeshStartScale)) (* _output_get (Variables|Default|GetMeshStartScale))) true :!class /Script/Engine.SplineMeshComponent))

(fn AddStaticMesh
  (params (RelativeLocation :type Vector) (Location :type Vector) (Rotation :type Rotator) (Scale :type Vector))
  (if (Variables|Default|GetUseStaticMesh)
    ;[1 1 1] AddWhateverChildActor
    (bind _returnvalue (AddComponent|AddStaticMeshComponent false (Math|Transform|MakeTransform "0, 0,0.000000" "0, 0, 0" (Math|Conversions|ToVector(Float) (Variables|Default|GetStaticMeshScale)))))
    (Components|StaticMesh|SetStaticMesh _returnvalue (Variables|Default|GetStaticMesh))
    (Rendering|Material|SetMaterial _returnvalue 0 (Variables|Default|GetStaticMeshMaterial))
    (Transformation|AttachComponentToComponent _returnvalue (Variables|Default|GetAs%20Spline%20Component) "None" "KeepRelative" "KeepRelative" "KeepRelative" true)
    (Transformation|SetWorldLocation _returnvalue (+ RelativeLocation Location) false false)
    (Transformation|SetRelativeRotation _returnvalue Rotation false false)
    (Transformation|SetRelativeScale3D _returnvalue Scale)))

(fn MeshRollSpline
  (params (SplineMeshComponent :type Spline%20Mesh%20Component%20Object%20Reference) (MeshSize :type Float%20%28double-precision%29))
  ;[1 1 1] Spline Roll
  (bind _output_get (Variables|Default|SetSplineRollStrength (Variables|Default|GetSplineRollStrength)))
  (Class|SplineMeshComponent|SetStartRoll SplineMeshComponent (* _output_get (Variables|Default|GetSplineRoll)) true)
  (bind _output_get_2 (Variables|Default|SetSplineRoll (- (Variables|Default|GetSplineRoll) (/ 1.0 (/ (Spline|GetSplineLength (Variables|Default|GetAs%20Spline%20Component)) MeshSize)))))
  (Class|SplineMeshComponent|SetEndRoll SplineMeshComponent (* _output_get_2 (Variables|Default|GetSplineRollStrength)) true))