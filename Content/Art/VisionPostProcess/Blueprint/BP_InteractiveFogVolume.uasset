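; BP_InteractiveFogVolume is a configurable volumetric fog actor, shaped by a volume texture, a 2D texture or a sphere.
; Its construction script creates a dynamic instance of M_VolumetricFog_Inst and passes it to the NSFogWhite Niagara component as FogMID.
; It then sets the textures, sphere size and extinction on that material, encoding the shape choice as a one-hot color vector.
; The event graph holds no runtime logic.
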(event EventBeginPlay)

(event Collision|EventActorBeginOverlap
  (params (OtherActor :type Actor%20Object%20Reference)))

(event EventTick
  (params (DeltaSeconds :type Float%20%28single-precision%29)))

(fn ConstructionScript
  (bind _returnvalue (Rendering|Material|CreateDynamicMaterialInstance "/Game/Art/VisionPostProcess/Material/M_VolumetricFog_Inst.M_VolumetricFog_Inst" "None" "None" :!class /Script/Engine.KismetMaterialLibrary))
  (bind _output_get (Variables|Default|SetFogMID _returnvalue))
  (Class|NiagaraComponent|SetVariableMaterial (Variables|Default|GetNS_FogWhite) "FogMID" _output_get)
  (Rendering|Material|SetVectorParameterValue (Variables|Default|GetFogMID) "ShapeType" (Utilities|Select :Index (Variables|BaseShape|GetShapeType) :NewEnumerator0 "(R=1.000000,G=0.000000,B=0.000000,A=0.000000)" :NewEnumerator1 "(R=0.000000,G=1.000000,B=0.000000,A=0.000000)" :NewEnumerator2 "(R=0.000000,G=0.000000,B=1.000000,A=0.000000)") :!class /Script/Engine.MaterialInstanceDynamic)
  (Rendering|Material|SetScalarParameterValue (Variables|Default|GetFogMID) "SphereSize" (Variables|BaseShape|GetSphereSize) :!class /Script/Engine.MaterialInstanceDynamic)
  (Rendering|Material|SetTextureParameterValue (Variables|Default|GetFogMID) "2D Texture" (Variables|BaseShape|GetTexture%202D))
  (Rendering|Material|SetTextureParameterValue (Variables|Default|GetFogMID) "VolumeTexture" (Variables|BaseShape|GetVolume%20Texture))
  (Rendering|Material|SetScalarParameterValue (Variables|Default|GetFogMID) "GlobalExtinction" (Variables|FogSettings|GetGlobalExtinction) :!class /Script/Engine.MaterialInstanceDynamic))